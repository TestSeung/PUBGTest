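; BP_Interactable is an item actor whose mesh is set from data, keyed by its ItemClassID.
; On BeginPlay, a non-zero ID is used as the row name in the ItemClassTable data table.
; The row's StaticMesh is async loaded, then applied to the StaticMeshComponent.
; ItemPicked is an empty function, so the file holds no pickup logic.
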(event EventBeginPlay
  ;[1 1 1] 예외처리
  (if (!= (Variables|Default|GetItemClassID) 0)
    (bind _returnvalue (Utilities|GetDataTableRow "/Game/Bluprints/Item/ItemClassTable.ItemClassTable" (Utilities|String|StringToName (Utilities|String|ToString(Integer) (Variables|Default|GetItemClassID))))
      (:then
        (bind _object (Utilities|AsyncLoadAsset (.StaticMesh (Utilities|Struct|BreakItemClass _returnvalue)))
          (:Completed
            (bind _as스태틱_메시 (Utilities|Casting|CastToStaticMesh _object))
            (Components|StaticMesh|SetStaticMesh (Variables|Default|GetStaticMeshComponent) _as스태틱_메시)))))))

(fn ConstructionScript)

(fn ItemPicked)